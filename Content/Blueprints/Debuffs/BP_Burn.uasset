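; BP_Burn is a burn debuff for turn-based characters that deals damage over several turns.
; At the start of each turn it applies a fixed amount of magic damage to the debuffed character and decrements its counter.
; When the counter runs out, it removes itself from that character's debuff list.
; The apply and end-of-turn hooks only print debug strings, with apply also returning zero.
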(event `self.OnBeginTurnWithDebuff`
  (params (Grid :type "GridManagerActor Object Reference"))
  (`KismetSystemLibrary.PrintString` null "OnFire Begin Turn")
  (`GameplayCharacter.MyTakeDamage` (`self.DebuffedCharacter`) 5.0 "MAGIC")
  (bind _result (`/Engine/EditorBlueprintResources/StandardMacros.DecrementInt` (`self.Counter`))
    (:`  `
      (if (<= _result 0)
        (`KismetArrayLibrary.Array_RemoveItem` (`GameplayCharacter.Debuffs` (`self.DebuffedCharacter`)) self)))))

(event `self.OnEndTurnWithDebuff`
  (params (Grid :type "GridManagerActor Object Reference"))
  (`KismetSystemLibrary.PrintString` null "OnFire End Turn"))

(fn `OnDebuffApplyed`
  (params (Grid :type "GridManagerActor Object Reference") (InstigatingCharacter :type "GameplayCharacter Object Reference"))
  (returns (ReturnValue :type "Float (single-precision)"))
  (`KismetSystemLibrary.PrintString` null "OnFire")
  (return 0.0))