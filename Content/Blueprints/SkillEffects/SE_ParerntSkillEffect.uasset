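; SE_ParerntSkillEffect is the parent Blueprint for skill effects in a tile-targeted skill system.
; PlaySkillEffect takes the user, targeted tile, skill and targets, and is a stub returning zero, apparently for child effects to override.
; Helper functions add and subtract two-component X/Y vectors component-wise, and another prints one as a comma-separated string for debugging.
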(fn `AddVectors`
  (params (vector1 :type "IntVector2 Structure") (vector2 :type "IntVector2 Structure"))
  (returns (Sum :type "IntVector2 Structure"))
  (return (make `IntVector2` (+ vector1_X vector2_X) (+ vector1_Y vector2_Y))))

(fn `PlaySkillEffect`
  (params (SkillUser :type "GameplayCharacter Object Reference") (targetedTile :type "IntVector2 Structure") (skillUsed :type "SkillDefinition Structure") (Targets :type "Array of GameplayCharacter Object Reference (by ref)"))
  (returns (ReturnValue :type "Float (single-precision)"))
  (return 0.0))

(fn `PrintVector`
  (params (NewParam :type "IntVector2 Structure"))
  (`KismetSystemLibrary.PrintString` null (`KismetStringLibrary.Concat_StrStr` (`KismetStringLibrary.Conv_IntToString` NewParam_X) "," (`KismetStringLibrary.Conv_IntToString` NewParam_Y))))

(fn `SubVectors`
  (params (Vector1 :type "IntVector2 Structure") (Vector2 :type "IntVector2 Structure"))
  (returns (OutVector :type "IntVector2 Structure"))
  (return (make `IntVector2` (- Vector1_X Vector2_X) (- Vector1_Y Vector2_Y))))